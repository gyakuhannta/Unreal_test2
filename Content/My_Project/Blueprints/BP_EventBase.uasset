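; BP_EventBase is a base Blueprint for game events whose completion status persists through BP_MyGameinstance.
; The construction script derives the EventName key from the object's display name.
; On BeginPlay it looks up that key's status, re-applying Finished through SetEventFinished or otherwise saving it as Unfinished.
; SetEventFinished marks the event Finished and writes that status back to the game instance.
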(event `self.ReceiveBeginPlay`
  (bind _asbp_my_gameinstance (cast `/Game/My_Project/Blueprints/BP_MyGameinstance` (`GameplayStatics.GetGameInstance`)))
  (bind _output_get (set `self.MyGameInstance` _asbp_my_gameinstance))
  (bind _output_get_2 (set `self.EventStatus` (`/Game/My_Project/Blueprints/BP_MyGameinstance.GatEventStatus` _output_get (`self.EventName`))))
  (switch `/Game/My_Project/Blueprints/EN_EventStatus` _output_get_2
    (:`NewEnumerator0`
      (bind _output_get_3 (set `self.EventStatus` "NewEnumerator1"))
      (`/Game/My_Project/Blueprints/BP_MyGameinstance.SaveEventStatus` (`self.MyGameInstance`) (`self.EventName`) _output_get_3))
    (:`NewEnumerator2`
      (`self.SetEventFinished`))))

(fn `SetEventFinished`
  (bind _output_get (set `self.EventStatus` "NewEnumerator2"))
  (`/Game/My_Project/Blueprints/BP_MyGameinstance.SaveEventStatus` (`self.MyGameInstance`) (`self.EventName`) _output_get))

(fn `UserConstructionScript`
  (set `self.EventName` (`KismetStringLibrary.Conv_StringToName` (`KismetSystemLibrary.GetDisplayName` self))))